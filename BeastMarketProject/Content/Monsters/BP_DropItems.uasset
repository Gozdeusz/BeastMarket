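; Monster loot helper that spawns item actors from a supplied list of dropped items at a set location.
; For each entry it rolls quality upgrades, a drop chance and extra quantity, with upgrade and extra-item chances halving after each success.
; Dropped items get price multiplied by quality and spawn with random horizontal scatter.
; Working stats and chances reset only after a successful spawn, so reduced quality odds carry past failed drops.
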(event Custom|SetDroppedItems
  (params (DroppedItems :type Array%20of%20S%20Slot%20Structures))
  (Variables|Default|SetDroppedItems DroppedItems))

(event Custom|DropItems
  (bind _spawnlocation (Variables|Default|GetSpawnLocation))
  (for _array_element (Variables|Default|GetDroppedItems)
    (CallFunction|SetStats (.quality (.uniquevalues _array_element)) (.quantity (.uniquevalues _array_element)) (.price (.uniquevalues _array_element)))
    ;[1 1 1] Quality
    (while (<= (* (Math|Random|RandomFloat) 1e+02) (Variables|Default|GetBetterQualityChance))
      (Variables|Default|SetQuality (+ (Variables|Default|GetQuality) 1))
      (if (<= (Variables|Default|GetBetterQualityChance) 5.0)
        (Variables|Default|SetBetterQualityChance 0.0)
        (else
          (Variables|Default|SetBetterQualityChance (/ (Variables|Default|GetBetterQualityChance) 2.0)))))
    ;[1 1 1] Quantity
    (if (<= (Math|Random|RandomFloatinRange 0.0 1e+02) (Variables|Default|GetDropChance))
      (while (<= (Math|Random|RandomFloatinRange 0.0 1e+02) (Variables|Default|GetAdditionalItemChance))
        (Variables|Default|SetQuantity (+ (Variables|Default|GetQuantity) 1))
        (if (<= (Variables|Default|GetAdditionalItemChance) 1.0)
          (Variables|Default|SetAdditionalItemChance 0.0)
          (else
            (Variables|Default|SetAdditionalItemChance (/ (Variables|Default|GetAdditionalItemChance) 2.0)))))
      ;[1 1 1] Price
      (Variables|Default|SetPrice (* (Variables|Default|GetPrice) (Variables|Default|GetQuality)))
      (Game|SpawnActorfromClass "/Game/Equipment/BP_Item.BP_Item_C" (Math|Transform|MakeTransform (Math|Vector|MakeVector (+ (.x _spawnlocation) (* (Math|Random|RandomFloatinRange -1.0 1.0) (Variables|Default|GetRandLocationAdjust))) (+ (.y _spawnlocation) (* (Math|Random|RandomFloatinRange -1.0 1.0) (Variables|Default|GetRandLocationAdjust))) (.z _spawnlocation)) "0, 0, 0" "1.000000,1.000000,1.000000") "AdjustIfPossibleButAlwaysSpawn" "MultiplyWithRoot" 0 (Utilities|Struct|MakeS_Slot (.item _array_element) (Utilities|Struct|MakeS_UniqueItemValues (Variables|Default|GetQuality) (Variables|Default|GetQuantity) (Variables|Default|GetPrice))) (Utilities|Struct|MakeS_UniqueItemValues (Variables|Default|GetQuality) (Variables|Default|GetQuantity) (Variables|Default|GetPrice)) 0)
      (CallFunction|ClearStats))))

(event Custom|PrintItem
  (params (S_Slot :type S%20Slot%20Structure%20%28by%20ref%29))
  ;[1 1 0] Debug
  (Development|PrintString (Utilities|String|Append "Item: " (Utilities|GetDisplayName (.datatable (.item S_Slot))) " Quality: " (Utilities|String|ToString(Integer) (.quality (.uniquevalues S_Slot))) " Quantity: " (Utilities|String|ToString(Integer) (.quantity (.uniquevalues S_Slot))) " Price: " (Utilities|String|ToString(Float) (.price (.uniquevalues S_Slot)))) true true "(R=1.000000,G=0.000000,B=1.000000,A=1.000000)" 15.0))

(event Custom|SetStats
  (params (Quality :type Integer) (Quantity :type Integer) (Price :type Float%20%28double-precision%29))
  (Variables|Default|SetQuality Quality)
  (Variables|Default|SetQuantity Quantity)
  (Variables|Default|SetPrice Price))

(event Custom|ClearStats
  (Variables|Default|SetQuality 0)
  (Variables|Default|SetQuantity 0)
  (Variables|Default|SetPrice 0.0)
  (Variables|Default|SetAdditionalItemChance 5e+01)
  (Variables|Default|SetBetterQualityChance 5e+01))

(event Custom|SetDropLocation
  (params (SpawnLocation :type Vector))
  (Variables|Default|SetSpawnLocation SpawnLocation))