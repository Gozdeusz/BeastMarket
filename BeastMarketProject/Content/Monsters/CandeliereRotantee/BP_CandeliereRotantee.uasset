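; Rotating-candelabrum monster, a PaperZD sprite enemy that chases and attacks the player and flips to face its movement.
; LookRange overlaps toggle sight and HP bar; Tick-driven CheckStatus uses AIMoveTo to chase, then play Attack, or return to spawn after losing sight.
; AnyDamage subtracts Defense (minimum one HP lost), briefly blocking further hits and movement.
; Animation state jumps show attack, hurt and death, which drops items before destroying the actor.
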(event OnComponentBeginOverlap(LookRange)
  (params (OverlappedComponent :type Primitive%20Component%20Object%20Reference) (OtherActor :type Actor%20Object%20Reference) (OtherComp :type Primitive%20Component%20Object%20Reference) (OtherBodyIndex :type Integer) (bFromSweep :type Boolean) (SweepResult :type Hit%20Result%20Structure%20%28by%20ref%29))
  ;[1 1 1] Following and Attacking Player
  (Utilities|Casting|CastToBP_MCH OtherActor)
  (Variables|Default|SetIsSeeingPlayer true)
  (CallFunction|ShowHPBar))

(event OnComponentEndOverlap(LookRange)
  (params (OverlappedComponent :type Primitive%20Component%20Object%20Reference) (OtherActor :type Actor%20Object%20Reference) (OtherComp :type Primitive%20Component%20Object%20Reference) (OtherBodyIndex :type Integer))
  ;[1 1 1] Following and Attacking Player
  (Utilities|Casting|CastToBP_MCH OtherActor)
  (Variables|Default|SetIsSeeingPlayer false)
  (CallFunction|HideHPBar))

(event Custom|Rotation
  (params (DeltaSeconds :type Float%20%28single-precision%29))
  ;[1 1 1] Rotation
  (|CallParentFunction DeltaSeconds)
  (if (not (Variables|Default|GetIsAttacking))
    (Math|Float|CompareFloat (.X (Math|Vector|BreakVector (Variables|/Script/Engine.MovementComponent|GetVelocity (Pawn|GetMovementComponent)))) 0.0
      (:>
        ;;[0 0.4745 1] Look Left
        (Utilities|IsValid (Pawn|GetController) :!label _label
          (:Is%20Valid
            (Transformation|SetWorldRotation (Variables|Default|GetSprite) (Math|Rotator|MakeRotator 0.0 0.0 1.8e+02) false false)
            (Variables|Default|SetIsLeft true))))
      (:==
        (if (Variables|Default|GetIsLeft)
          (goto _label)
          (else
            ;;[0 0.4745 1] Look Right
            (Utilities|IsValid (Pawn|GetController) :!label _label_2
              (:Is%20Valid
                (Transformation|SetWorldRotation (Variables|Default|GetSprite) (Math|Rotator|MakeRotator 0.0 0.0 0.0) false false)
                (Variables|Default|SetIsLeft false))))))
      (:<
        (goto _label_2)))))

(event Custom|CheckStatus
  (bind _self self)
  ;[1 1 1] BackToStartPosition
  (if (not (Variables|Default|GetDoing))
    (if (not (Variables|Default|GetIsAttacking))
      (if (Variables|Default|GetIsSeeingPlayer)
        (if (not (Variables|Default|GetIsMovementLocked))
          (Variables|Default|SetDoing true)
          (Utilities|FlowControl|DoOnce false :!label _label
            (:Completed
              (Utilities|FlowControl|Delay 0.2)
              (if (Variables|Default|GetIsMovementLocked)
                _
                (else
                  (CallFunction|FollowPlayer)))
              (Variables|Default|SetDoing false)
              (goto _label Reset))))
        (else
          (Variables|Default|SetDoing true)
          (Utilities|FlowControl|DoOnce false :!label _label_2
            (:Completed
              (Utilities|FlowControl|Delay 0.01)
              (AI|AIMoveTo _self (Transformation|GetActorLocation _self) 0 75.0 false
                (:then
                  (Utilities|FlowControl|Delay 5.0)
                  (AI|AIMoveTo self (Variables|Default|GetStandPositon) 0 75.0 false
                    (:OnSuccess
                      (Variables|Default|SetDoing false)
                      (goto _label_2 Reset))))))))))))

(event Custom|ShowHPBar
  ;[1 1 1] HPBar
  (bind _aswb_hpbar (Utilities|Casting|CastToWB_HPBar (UserInterface|GetWidget (Variables|Default|GetHPBar))))
  (Variables|/Script/UMG.UserWidget|SetColorAndOpacity _aswb_hpbar (Utilities|Struct|MakeLinearColor (.r (Variables|/Script/UMG.UserWidget|GetColorAndOpacity _aswb_hpbar)) (.g (Variables|/Script/UMG.UserWidget|GetColorAndOpacity _aswb_hpbar)) (.b (Variables|/Script/UMG.UserWidget|GetColorAndOpacity _aswb_hpbar)) 1.0)))

(event Custom|FollowPlayer
  ;[1 1 1] Following and Attacking Player
  (AI|AIMoveTo self "0, 0, 0" (Game|GetPlayerCharacter 0) 75.0 (Variables|Default|GetIsSeeingPlayer)
    (:OnSuccess
      (Utilities|FlowControl|Delay 0.01)
      (Utilities|FlowControl|DoOnce false :!label _label
        (:Completed
          (Variables|Default|SetIsAttacking true)
          (Variables|Default|SetIsMovementLocked true)
          (Class|BPIStateRequest|JumpStateRequest(Message) (Variables|/Script/PaperZD.PaperZDAnimationComponent|GetAnimInstance (Variables|Default|GetAnimationComponent)) "Attack" "Locomotion")
          (Utilities|FlowControl|Delay (Variables|Default|GetDelayAfterAttack))
          (Variables|Default|SetIsAttacking false)
          (Variables|Default|SetIsMovementLocked false)
          (goto _label Reset))))))

(event Custom|HideHPBar
  ;[1 1 1] HPBar
  (bind _aswb_hpbar (Utilities|Casting|CastToWB_HPBar (UserInterface|GetWidget (Variables|Default|GetHPBar))))
  (Variables|/Script/UMG.UserWidget|SetColorAndOpacity _aswb_hpbar (Utilities|Struct|MakeLinearColor (.r (Variables|/Script/UMG.UserWidget|GetColorAndOpacity _aswb_hpbar)) (.g (Variables|/Script/UMG.UserWidget|GetColorAndOpacity _aswb_hpbar)) (.b (Variables|/Script/UMG.UserWidget|GetColorAndOpacity _aswb_hpbar)) 0.0)))

(event Custom|RefreshHPBar
  ;[1 1 1] HPBar
  (bind _aswb_hpbar (Utilities|Casting|CastToWB_HPBar (UserInterface|GetWidget (Variables|Default|GetHPBar))))
  (Progress|SetPercent (Variables|/Game/Monsters/WB_HPBar.WB_HPBar_C|GetHP_Bar _aswb_hpbar) (/ (Math|Conversions|ToFloat(Integer) (.health (Variables|Default|GetStats))) 1e+02)))

(event Game|Damage|EventAnyDamage
  (params (Damage :type Float%20%28single-precision%29) (DamageType :type Damage%20Type%20Object%20Reference) (InstigatedBy :type Controller%20Object%20Reference) (DamageCauser :type Actor%20Object%20Reference))
  (bind _animationcomponent (Variables|Default|GetAnimationComponent))
  (bind _animinstance (Variables|/Script/PaperZD.PaperZDAnimationComponent|GetAnimInstance _animationcomponent))
  ;[1 1 1] DMG / DEF System
  (Variables|Default|SetIsMovementLocked true)
  (if (Variables|Default|GetCanBeDamaged)
    (Variables|Default|SetbCanBeDamaged false)
    (if (>= (.defense (Variables|Default|GetStats)) Damage)
      (bind _output_get (Variables|Default|SetStats (Utilities|Struct|MakeS_BaseEnemyStats (- (.health (Variables|Default|GetStats)) 1) (.attackdamage (Variables|Default|GetStats)) (.defense (Variables|Default|GetStats)) (.level (Variables|Default|GetStats)))))
      ;;[1 1 0] Debug Only
      (Development|PrintString (Utilities|String|Append (Utilities|GetObjectName self) " HP = " (Utilities|String|ToString(Integer) (.health _output_get))) true true "(R=0.040787,G=1.000000,B=0.000000,A=1.000000)")
      (else
        (bind _output_get_2 (Variables|Default|SetStats (Utilities|Struct|MakeS_BaseEnemyStats (- (.health (Variables|Default|GetStats)) (- Damage (.defense (Variables|Default|GetStats)))) (.attackdamage (Variables|Default|GetStats)) (.defense (Variables|Default|GetStats)) (.level (Variables|Default|GetStats)))))
        (Development|PrintString (Utilities|String|Append (Utilities|GetObjectName self) " HP = " (Utilities|String|ToString(Integer) (.health _output_get_2))) true true "(R=0.040787,G=1.000000,B=0.000000,A=1.000000)")))
    (if (or (<= (.health _output_get) 0) (<= (.health _output_get_2) 0))
      (Class|BPIStateRequest|JumpStateRequest(Message) _animinstance "Dead" "Locomotion")
      (Utilities|FlowControl|Delay 0.5)
      (Default|SetDropLocation (Variables|Default|GetBP_DropItems) (Transformation|GetActorLocation))
      (Default|DropItems (Variables|Default|GetBP_DropItems))
      (Utilities|FlowControl|Delay 0.5)
      (Actor|DestroyActor)
      (Variables|Default|SetIsMovementLocked false)
      (else
        (Class|BPIStateRequest|JumpStateRequest(Message) _animinstance "Damaged" "Locomotion")
        (Utilities|FlowControl|Delay 0.5)
        (Variables|Default|SetbCanBeDamaged true)
        (Variables|Default|SetIsMovementLocked false)))))

(event EventTick
  (params (DeltaSeconds :type Float%20%28single-precision%29))
  (CallFunction|Rotation DeltaSeconds)
  (CallFunction|RefreshHPBar)
  (Utilities|FlowControl|DoOnce false :!label _label
    (:Completed
      (CallFunction|CheckStatus)
      (goto _label Reset))))

(event EventBeginPlay
  (Variables|Default|SetStandPositon (Transformation|GetActorLocation self))
  (CallFunction|HideHPBar)
  (Default|SetDroppedItems (Variables|Default|GetBP_DropItems) (Variables|Default|GetDroppedItems)))

(fn ConstructionScript)