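; Main player character with planar movement, left/right facing, a timeline-driven dash, light/heavy combo attacks, and interactions for level swapping and crafting.
; Movement lock and shop/fight mode flags gate actions, while state-machine jumps and combo messages drive the animation instance.
; Damage subtracts Defense (minimum one), grants brief invulnerability, and shows Game Over at zero health.
; Save helpers pack and restore transform, stats, equipment and level name.
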(event Custom|SwapToFightMode
  (Development|PrintString "FightMode")
  (Variables|Default|SetIsShopMode false))

(event Custom|SwapToShopMode
  (Development|PrintString "ShopMode")
  (Variables|Default|SetIsShopMode true))

(event Game|Damage|EventAnyDamage
  (params (Damage :type Float%20%28single-precision%29) (DamageType :type Damage%20Type%20Object%20Reference) (InstigatedBy :type Controller%20Object%20Reference) (DamageCauser :type Actor%20Object%20Reference))
  (bind _returnvalue (Game|GetPlayerController 0))
  ;[1 1 1] DMG / DEF System
  (if (and (Variables|Default|GetbCanBeDamaged) (not (Variables|Default|GetIsShopMode)))
    (Variables|Default|SetbCanBeDamaged false)
    (if (>= (.defense (Variables|Default|GetStats)) Damage)
      (bind _output_get (Variables|Default|SetStats (Utilities|Struct|MakeS_BaseStats (- (.health (Variables|Default|GetStats)) 1) (.attack_damage (Variables|Default|GetStats)) (.defense (Variables|Default|GetStats)) (.weight (Variables|Default|GetStats)) (.money (Variables|Default|GetStats)) (.stamina (Variables|Default|GetStats)) (.experience (Variables|Default|GetStats)) (.level (Variables|Default|GetStats)))))
      ;;[1 1 0] Debug only
      (Development|PrintString (Utilities|String|ToString(Integer) (.health _output_get)) true true "(R=0.000000,G=1.000000,B=0.000000,A=1.000000)" 3.0)
      (else
        (bind _output_get_2 (Variables|Default|SetStats (Utilities|Struct|MakeS_BaseStats (- (.health (Variables|Default|GetStats)) (- Damage (.defense (Variables|Default|GetStats)))) (.attack_damage (Variables|Default|GetStats)) (.defense (Variables|Default|GetStats)) (.weight (Variables|Default|GetStats)) (.money (Variables|Default|GetStats)) (.stamina (Variables|Default|GetStats)) (.experience (Variables|Default|GetStats)) (.level (Variables|Default|GetStats)))))
        ;;[1 1 0] Debug only
        (Development|PrintString (Utilities|String|ToString(Integer) (.health _output_get_2)) true true "(R=0.000000,G=1.000000,B=0.000000,A=1.000000)" 3.0)))
    (if (or (<= (.health _output_get) 0) (<= (.health _output_get_2) 0))
      (Class|BPIStateRequest|JumpStateRequest(Message) (Variables|/Script/PaperZD.PaperZDAnimationComponent|GetAnimInstance (Variables|Default|GetAnimationComponent)) "Dead" "Locomotion")
      ;;[0.1385 0 1] ADD_DEATH_WIDGET_HERE
      (bind _returnvalue_2 (UserInterface|CreateWidget "/Game/Blueprints/WB_GameOver.WB_GameOver_C"))
      (UserInterface|Viewport|AddtoViewport _returnvalue_2 0)
      (UserInterface|Animation|PlayAnimation _returnvalue_2 (Variables|/Game/Blueprints/WB_GameOver.WB_GameOver_C|GetFadeAnimation _returnvalue_2) 0.0 1 "Forward" 1.0 false)
      (Variables|/Script/Engine.PlayerController|SetbShowMouseCursor _returnvalue true)
      (Input|SetInputModeGameandUI _returnvalue _returnvalue_2 "DoNotLock" true false)
      (Utilities|FlowControl|Delay 2.5)
      (Variables|Default|SetbCanBeDamaged true)
      (else
        (Class|BPIStateRequest|JumpStateRequest(Message) (Variables|/Script/PaperZD.PaperZDAnimationComponent|GetAnimInstance (Variables|Default|GetAnimationComponent)) "Damaged" "Locomotion")
        (Utilities|FlowControl|Delay 1.0)
        (Variables|Default|SetbCanBeDamaged true)))))

(event EventBeginPlay
  (Rendering|SceneCapture|ShowOnlyActorComponents (Variables|Default|GetModelSCC2D) self false))

(event EventTick
  (params (DeltaSeconds :type Float%20%28single-precision%29))
  (bind _returnvalue (Pawn|GetController))
  (bind _returnvalue_2 (Pawn|GetController))
  ;[1 1 1] Rotation
  (|CallParentFunction DeltaSeconds)
  (Math|Float|CompareFloat (.X (Math|Vector|BreakVector (Variables|/Script/Engine.MovementComponent|GetVelocity (Pawn|GetMovementComponent)))) 0.0
    (:>
      ;;[0 0.4745 1] Look Right
      (Utilities|IsValid _returnvalue_2
        (:Is%20Valid
          (Pawn|SetControlRotation _returnvalue_2 (Math|Rotator|MakeRotator 0.0 0.0 0.0)))))
    (:<
      ;;[0 0.4745 1] Look Left
      (Utilities|IsValid _returnvalue
        (:Is%20Valid
          (Pawn|SetControlRotation _returnvalue (Math|Rotator|MakeRotator 0.0 0.0 1.8e+02)))))))

(event EventOnWalkingOffLedge
  (params (PreviousFloorImpactNormal :type Vector%20%28by%20ref%29 :default "0, 0, 0") (PreviousFloorContactNormal :type Vector%20%28by%20ref%29 :default "0, 0, 0") (PreviousLocation :type Vector%20%28by%20ref%29 :default "0, 0, 0") (TimeDelta :type Float%20%28single-precision%29))
  ;[1 1 1] Dashing
  (Class|PaperZDAnimInstance|JumptoNode (Variables|/Script/PaperZD.PaperZDAnimationComponent|GetAnimInstance (Variables|Default|GetAnimationComponent)) "InAir" "Locomotion"))

(event EventOnLanded
  (params (Hit :type Hit%20Result%20Structure%20%28by%20ref%29))
  ;[1 1 1] Dashing
  (Class|PaperZDAnimInstance|JumptoNode (Variables|/Script/PaperZD.PaperZDAnimationComponent|GetAnimInstance (Variables|Default|GetAnimationComponent)) "Landed" "Locomotion"))

(event EventOnJumped
  ;[1 1 1] Dashing
  (Class|PaperZDAnimInstance|JumptoNode (Variables|/Script/PaperZD.PaperZDAnimationComponent|GetAnimInstance (Variables|Default|GetAnimationComponent)) "InAir" "Locomotion"))

(event Input|ActionEvents|InputActionInteraction
  (params (Key :type Key%20Structure :default "None"))
  (bind _returnvalue (Game|GetPlayerController 0))
  (:Pressed
    (if (Variables|Default|GetIsCraftingBoardRange?)
      (Variables|Default|SetIsMovementLocked false)
      (bind _returnvalue_2 (UserInterface|CreateWidget "/Game/Equipment/UI_Blueprints/CraftingPanel/WB_CraftingPanel.WB_CraftingPanel_C"))
      (UserInterface|Viewport|AddtoViewport _returnvalue_2 0)
      (Input|SetInputModeUIOnly _returnvalue _returnvalue_2 "DoNotLock" false)
      (Variables|/Script/Engine.PlayerController|SetbShowMouseCursor _returnvalue true))))

(event Input|ActionEvents|InputActionAttack_Light
  (params (Key :type Key%20Structure :default "None"))
  ;[1 1 1] ComboAttacks
  (:Pressed
    (if (and (not (Variables|Default|GetIsShopMode)) (not (Variables|Default|GetIsMovementLocked)))
      (Variables|Default|SetIsMovementLocked true)
      (Class|BPIComboRequest|RequestCombo(Message) (Variables|/Script/PaperZD.PaperZDAnimationComponent|GetAnimInstance (Variables|Default|GetAnimationComponent)) "NewEnumerator0")
      (Utilities|FlowControl|Delay 0.8)
      (Variables|Default|SetIsMovementLocked false))))

(event Input|ActionEvents|InputActionAttack_Heavy
  (params (Key :type Key%20Structure :default "None"))
  ;[1 1 1] ComboAttacks
  (:Pressed
    (if (and (not (Variables|Default|GetIsShopMode)) (not (Variables|Default|GetIsMovementLocked)))
      (Variables|Default|SetIsMovementLocked true)
      (Class|BPIComboRequest|RequestCombo(Message) (Variables|/Script/PaperZD.PaperZDAnimationComponent|GetAnimInstance (Variables|Default|GetAnimationComponent)) "NewEnumerator1")
      (Utilities|FlowControl|Delay 0.8)
      (Variables|Default|SetIsMovementLocked false))))

(event Input|ActionEvents|InputActionDash
  (params (Key :type Key%20Structure :default "None"))
  (bind _returnvalue (Transformation|GetVelocity))
  (bind _returnvalue_2 (Transformation|GetActorForwardVector))
  (bind _dashpower (Variables|Default|GetDashPower))
  (bind _returnvalue_3 (* _returnvalue_2 _dashpower))
  ;[1 1 1] Dashing
  (:Pressed
    (if (not (Variables|Default|GetIsShopMode))
      (if (not (Variables|Default|GetIsMovementLocked))
        (if (or (!= (.x _returnvalue) 0.0) (!= (.y _returnvalue) 0.0))
          (if (not (Variables|Default|GetIsDashing))
            (Variables|Default|SetbCanBeDamaged false)
            (Variables|Default|SetIsDashing true)
            (Class|BPIStateRequest|JumpStateRequest(Message) (Variables|/Script/PaperZD.PaperZDAnimationComponent|GetAnimInstance (Variables|Default|GetAnimationComponent)) "Dash" "Locomotion")
            (Timeline|Dash PlayFromStart
              (:Update
                (Variables|/Script/Engine.MovementComponent|SetVelocity (Variables|Character|GetCharacterMovement) (Math|Vector|MakeVector (.x _returnvalue_3) (.y _returnvalue_3) 0.0)))
              (:Finished
                (Variables|Default|SetbCanBeDamaged true)
                (Utilities|FlowControl|Delay (Variables|Default|GetDashCooldown))
                (Variables|Default|SetIsDashing false)))))))))

(event Input|ActionEvents|InputActionInteraction
  (params (Key :type Key%20Structure :default "None"))
  (:Pressed
    (if (Variables|Default|GetisOutDoors?)
      (bind _asbp_gmtest (Utilities|Casting|CastToBP_GMTest (Game|GetGameMode)))
      (Default|SwapLevel _asbp_gmtest "/Game/Levels/MainMap.MainMap")
      (Transformation|SetActorLocation "-7430.000000,9640.000000,1645.000000" false false))))

(event Input|AxisEvents|InputAxisRight/Left
  (params (AxisValue :type Float%20%28single-precision%29))
  ;[1 1 1] Movement
  (if (not (Variables|Default|GetIsMovementLocked))
    (Pawn|Input|AddMovementInput "1.000000,0.000000,0.000000" AxisValue false)))

(event Input|AxisEvents|InputAxisForward/Backward
  (params (AxisValue :type Float%20%28single-precision%29))
  ;[1 1 1] Movement
  (if (not (Variables|Default|GetIsMovementLocked))
    (Pawn|Input|AddMovementInput "0.000000,1.000000,0.000000" AxisValue false)))

(event Input|KeyboardEvents|DebugKeyX
  (params (Key :type Key%20Structure :default "None") (ActionValue :type Input%20Action%20Value%20Structure))
  (:Pressed
    (CallFunction|SwaptoFightMode)))

(event Input|KeyboardEvents|DebugKeyC
  (params (Key :type Key%20Structure :default "None") (ActionValue :type Input%20Action%20Value%20Structure))
  (:Pressed
    (CallFunction|SwaptoShopMode)))

(fn ConstructionScript)

(fn GetPlayerData
  (bind _bpc_equipmentsystem (Variables|Default|GetBPC_EquipmentSystem))
  (bind _returnvalue (Game|GetCurrentLevelName true))
  (return (Utilities|Struct|MakeS_PlayerSave (Transformation|GetActorTransform) (Variables|Default|GetStats) (Variables|/Game/Equipment/BPC_EquipmentSystem.BPC_EquipmentSystem_C|GetitemSlots _bpc_equipmentsystem) (Variables|/Game/Equipment/BPC_EquipmentSystem.BPC_EquipmentSystem_C|GetEquippedItems _bpc_equipmentsystem) _returnvalue)))

(fn UsePlayerSave
  (params (PlayerSave :type S%20Player%20Save%20Structure))
  (bind _bpc_equipmentsystem (Variables|Default|GetBPC_EquipmentSystem))
  (Game|OpenLevel(byName) (Utilities|String|StringToName (.currentlevel PlayerSave)))
  (Transformation|SetActorTransform (.transform PlayerSave))
  (Variables|Default|SetStats (.playerstats PlayerSave))
  (Variables|/Game/Equipment/BPC_EquipmentSystem.BPC_EquipmentSystem_C|SetitemSlots _bpc_equipmentsystem (.equipment PlayerSave))
  (Variables|/Game/Equipment/BPC_EquipmentSystem.BPC_EquipmentSystem_C|SetEquippedItems _bpc_equipmentsystem (.equippeditems PlayerSave)))