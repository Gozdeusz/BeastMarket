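; AC_Time is a component in the main character folder that runs a day/night cycle timer.
; Tick accumulates time scaled by TimeSpeed and compares it to the day or night length, both set in minutes.
; When a phase ends, TimeSwap flips IsDay and resets the timer, then a colored Polish debug message announces the change.
; A separate TimeStop/Start event toggles pausing of the clock.
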(event Custom|TimeSwap
  (if (Variables|Default|GetIsDay)
    (Variables|Default|SetIsDay false)
    (Variables|Default|SetTime 0.0)
    (else
      (Variables|Default|SetIsDay true)
      (Variables|Default|SetTime 0.0))))

(event Custom|TimeStop/Start
  (if (Variables|Default|GetStopTime)
    (Variables|Default|SetStopTime false)
    (else
      (Variables|Default|SetStopTime true))))

(event EventTick
  (params (DeltaSeconds :type Float%20%28single-precision%29))
  (if (not (Variables|Default|GetStopTime))
    (Variables|Default|SetTime (+ (* DeltaSeconds (Variables|Default|GetTimeSpeed)) (Variables|Default|GetTime)))
    (if (Variables|Default|GetIsDay)
      (if (>= (Variables|Default|GetTime) (* (Variables|Default|GetDayTime) 6e+01))
        (CallFunction|TimeSwap)
        (Development|PrintString "Koniec Dnia!" true true "(R=0.954491,G=1.000000,B=0.000000,A=1.000000)" 3.0))
      (elif (>= (Variables|Default|GetTime) (* (Variables|Default|GetNightTime) 6e+01))
        (CallFunction|TimeSwap)
        (Development|PrintString "Koniec Nocy!" true true "(R=0.000000,G=0.209997,B=1.000000,A=1.000000)" 3.0)))))

(event EventBeginPlay
  (Variables|Default|SetTime 0.0))