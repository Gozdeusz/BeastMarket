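; BP_GMTest appears to be a test game mode that handles HUD creation and level switching.
; LoadHUD reads ModeType from BP_Gamestate, showing either the hunt stats widget or the shop widget, seeded with BP_MCH's money and the day number.
; SwapLevel adds a loading screen, opens the given level by reference, and removes the screen immediately after that call.
; BeginPlay is empty, so both events rely on external callers.
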(event Custom|SwapLevel
  (params (Level :type World%20Soft%20Object%20Reference))
  (bind _returnvalue (UserInterface|CreateWidget "/Game/Equipment/UI_Blueprints/WB_LoadingScreen.WB_LoadingScreen_C"))
  (UserInterface|Viewport|AddtoViewport _returnvalue 0)
  (Game|OpenLevel(byObjectReference) Level)
  (Widget|RemovefromParent _returnvalue))

(event Custom|LoadHUD
  (bind _asbp_gamestate (Utilities|Casting|CastToBP_Gamestate (Game|GetGameState)))
  (if (Variables|/Game/Blueprints/BP_Gamestate.BP_Gamestate_C|GetModeType _asbp_gamestate)
    (bind _asbp_mch (Utilities|Casting|CastToBP_MCH (Game|GetPlayerCharacter 0)))
    (bind _returnvalue (UserInterface|CreateWidget "/Game/Blueprints/WB_ShopMode.WB_ShopMode_C" 0 (Utilities|Text|ToText(Integer) (Utilities|Struct|BreakS_BaseStats (Variables|/Game/Blueprints/Main_Character/BP_MCH.BP_MCH_C|GetStats _asbp_mch))) (Utilities|Text|ToText(Integer) (Variables|/Game/Blueprints/BP_Gamestate.BP_Gamestate_C|GetDayNumber _asbp_gamestate))))
    (UserInterface|Viewport|AddtoViewport _returnvalue 0)
    (else
      (bind _returnvalue_2 (UserInterface|CreateWidget "/Game/Blueprints/WB_HuntModeStats.WB_HuntModeStats_C"))
      (UserInterface|Viewport|AddtoViewport _returnvalue_2 0))))

(event EventBeginPlay)

(fn ConstructionScript)