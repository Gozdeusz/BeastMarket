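; BP_NPC is a sprite-based NPC that wanders and visits stands it detects.
; Overlaps of the LookRange sphere with BP_InteractableForNPC set IsSeeingStand and store the stand's position.
; When idle, Tick picks between AI moves to that stand, with a printed greeting, or to random nearby points, using delays, DoOnce gates and a Doing flag for pacing.
; Tick also flips the sprite by X velocity, keeping the last facing when still.
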(event OnComponentBeginOverlap(LookRange)
  (params (OverlappedComponent :type Primitive%20Component%20Object%20Reference) (OtherActor :type Actor%20Object%20Reference) (OtherComp :type Primitive%20Component%20Object%20Reference) (OtherBodyIndex :type Integer) (bFromSweep :type Boolean) (SweepResult :type Hit%20Result%20Structure%20%28by%20ref%29))
  (bind _asbp_interactable_for_npc (Utilities|Casting|CastToBP_InteractableForNPC OtherActor))
  (Variables|Default|SetIsSeeingStand true)
  (bind _output_get (Variables|Default|SetLocation (Variables|/Game/Blueprints/NPC/BP_InteractableForNPC.BP_InteractableForNPC_C|GetLocation _asbp_interactable_for_npc)))
  (Variables|Default|SetPositionOfStand (Transformation|GetWorldLocation _output_get)))

(event OnComponentEndOverlap(LookRange)
  (params (OverlappedComponent :type Primitive%20Component%20Object%20Reference) (OtherActor :type Actor%20Object%20Reference) (OtherComp :type Primitive%20Component%20Object%20Reference) (OtherBodyIndex :type Integer))
  (Utilities|Casting|CastToBP_InteractableForNPC OtherActor)
  (Variables|Default|SetIsSeeingStand false))

(event Custom|Rotation
  (params (DeltaSeconds :type Float%20%28single-precision%29))
  ;[1 1 1] Rotation
  (|CallParentFunction DeltaSeconds)
  (Math|Float|CompareFloat (.X (Math|Vector|BreakVector (Variables|/Script/Engine.MovementComponent|GetVelocity (Pawn|GetMovementComponent)))) 0.0
    (:>
      ;;[0 0.4745 1] Look Right
      (Utilities|IsValid (Pawn|GetController) :!label _label
        (:Is%20Valid
          (Transformation|SetWorldRotation (Variables|Default|GetSprite) (Math|Rotator|MakeRotator 0.0 0.0 0.0) false false)
          (Variables|Default|SetIsLeft false))))
    (:==
      (if (not (Variables|Default|GetIsLeft))
        (goto _label)
        (else
          ;;[0 0.4745 1] Look Left
          (Utilities|IsValid (Pawn|GetController) :!label _label_2
            (:Is%20Valid
              (Transformation|SetWorldRotation (Variables|Default|GetSprite) (Math|Rotator|MakeRotator 0.0 0.0 1.8e+02) false false)
              (Variables|Default|SetIsLeft true))))))
    (:<
      (goto _label_2))))

(event Custom|CheckStatus
  (Utilities|FlowControl|DoOnce false :!label _label
    (:Completed
      (Variables|Default|SetDoing true)
      (AI|AIMoveTo self (Variables|Default|GetPositionOfStand) 0 25.0 false
        (:OnSuccess
          (Development|PrintString "Hello")
          (Utilities|FlowControl|Delay 3.0)
          (CallFunction|MoveRandomly)
          (Utilities|FlowControl|Delay 5.0)
          (goto _label Reset))))))

(event Custom|MoveRandomly
  (bind _lookrange (Variables|Default|GetLookRange))
  (bind _returnvalue (Transformation|GetWorldLocation _lookrange))
  (bind _sphereradius (Variables|/Script/Engine.SphereComponent|GetSphereRadius _lookrange))
  (bind _returnvalue_2 (/ _sphereradius 2.0))
  (bind _returnvalue_3 (Math|Conversions|ToVector(Float) _returnvalue_2))
  (bind _returnvalue_4 (Math|Random|RandomPointinBoundingBox _returnvalue _returnvalue_3))
  (Utilities|FlowControl|DoOnce false :!label _label
    (:Completed
      (Variables|Default|SetDoing true)
      (AI|AIMoveTo self (Math|Vector|MakeVector (.x _returnvalue_4) (.y _returnvalue_4) 0.0) 0 75.0 false
        (:OnSuccess
          _)
        (:OnFail
          _))
      (Utilities|FlowControl|Delay 2.0)
      (Variables|Default|SetDoing false)
      (goto _label Reset))))

(event EventTick
  (params (DeltaSeconds :type Float%20%28single-precision%29))
  (CallFunction|Rotation DeltaSeconds)
  (if (not (Variables|Default|GetDoing))
    (if (Variables|Default|GetIsSeeingStand)
      (CallFunction|CheckStatus)
      (else
        (CallFunction|MoveRandomly)))))

(event EventBeginPlay)

(fn ConstructionScript)