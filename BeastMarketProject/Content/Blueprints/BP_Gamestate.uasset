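; Game state Blueprint that tracks the day number and running stats for defeated enemies, collected items, sold items and earned money.
; Small functions update each counter, with the collected-item decrement guarded against going below zero.
; GetOptionsForSummary uses ModeType to return labeled text values for either the sales pair or the combat and collection pair.
; ClearAllStats resets the four stats but leaves the day number intact.
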(event EventBeginPlay)

(event EventTick
  (params (DeltaSeconds :type Float%20%28single-precision%29)))

(fn ConstructionScript)

(fn DefeatedEnemiesNumberIncrease
  (bind _result (Math|Integer|IncrementInt (Variables|Default|GetAllDefeatedEnemies))
    (:%20%20
      (Variables|Default|SetAllDefeatedEnemies _result))))

(fn SoldItemsNumberIncrease
  (bind _result (Math|Integer|IncrementInt (Variables|Default|GetAllSoldItems))
    (:%20%20
      (Variables|Default|SetAllSoldItems _result))))

(fn EarnedMoneyValueIncrease
  (params (EarnedMoneyValue :type Float%20%28double-precision%29))
  (Variables|Default|SetAllEarnedMoney (+ (Variables|Default|GetAllEarnedMoney) EarnedMoneyValue)))

(fn CollectedItemsNumberIncrease
  (bind _result (Math|Integer|IncrementInt (Variables|Default|GetAllItemsCollected))
    (:%20%20
      (Variables|Default|SetAllItemsCollected _result))))

(fn CollectedItemsNumberDecrease
  (if (> (Variables|Default|GetAllItemsCollected) 0)
    (Variables|Default|SetAllItemsCollected (- (Variables|Default|GetAllItemsCollected) 1))))

(fn GetOptionsforSummary
  (if (Variables|Default|GetModeType)
    (return "Sold Items" "Earned Money" (Utilities|Text|ToText(Integer) (Variables|Default|GetAllSoldItems)) (Utilities|Text|ToText(Float) (Variables|Default|GetAllEarnedMoney) "HalfToEven"))
    (else
      (return "Defeated Enemies" "Collected Items" (Utilities|Text|ToText(Integer) (Variables|Default|GetAllDefeatedEnemies)) (Utilities|Text|ToText(Integer) (Variables|Default|GetAllItemsCollected))))))

(fn ChangeDay
  (bind _result (Math|Integer|IncrementInt (Variables|Default|GetDayNumber))
    (:%20%20
      (Variables|Default|SetDayNumber _result))))

(fn ClearAllStats
  (Variables|Default|SetAllDefeatedEnemies 0)
  (Variables|Default|SetAllSoldItems 0)
  (Variables|Default|SetAllEarnedMoney 0.0)
  (Variables|Default|SetAllItemsCollected 0))