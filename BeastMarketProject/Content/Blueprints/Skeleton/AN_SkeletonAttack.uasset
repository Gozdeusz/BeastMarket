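; Anim notify that applies the skeleton enemy's melee hit damage at the moment it fires in an attack animation.
; It box-overlaps pawns at the SkeletonAttack1 socket, ignoring the owner, and damages BP_MCH targets by the skeleton's AttackDamage stat times DMGMultiplier.
; Without a valid owning instance, it instead draws a debug box of the same Extent at that socket to show the hit area.
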(fn OnReceiveNotify
  (params (OwningInstance :type Paper%20ZD%20Anim%20Instance%20Object%20Reference))
  (bind _returnvalue (Class|PaperZDAnimInstance|GetOwningActor OwningInstance))
  (bind _sequencerendercomponent (Variables|Default|GetSequenceRenderComponent))
  (bind _extent (Variables|Default|GetExtent))
  (bind _returnvalue_2 (Transformation|GetSocketLocation _sequencerendercomponent "SkeletonAttack1"))
  (Utilities|IsValid OwningInstance
    (:Is%20Valid
      (bind _asbp_skeleton (Utilities|Casting|CastToBP_Skeleton _returnvalue))
      (bind _outactors (Collision|BoxOverlapActors _returnvalue_2 _extent (Utilities|Array|MakeArray "ObjectTypeQuery3") 0 (Utilities|Array|MakeArray _returnvalue) :!class /Script/Engine.KismetSystemLibrary))
      (for _array_element _outactors
        (Utilities|Casting|CastToBP_MCH _array_element)
        (Game|Damage|ApplyDamage _array_element (Math|Conversions|ToFloat(Integer) (* (.attackdamage (Variables|/Game/Blueprints/Skeleton/BP_Skeleton.BP_Skeleton_C|GetStats _asbp_skeleton)) (Variables|Default|GetDMG_Multiplier))) 0 0)))
    (:Is%20Not%20Valid
      (Rendering|Debug|DrawDebugBox _returnvalue_2 _extent "(R=1.000000,G=0.000000,B=0.531100,A=1.000000)" "0, 0, 0" 2.0 0.0))))