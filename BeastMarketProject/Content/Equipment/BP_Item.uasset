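; BP_Item is a world item actor that shows its name and quantity when BP_MCH overlaps its sphere.
; The construction script sets the Paper2D sprite and name from the ItemData table row, scales sprite and sphere, and debug-prints quality, quantity and price.
; Overlap fills WB_ItemInfo through SetItemInfo, showing quantity only above one, and plays UpAnimation.
; Leaving plays it in reverse, then hides the widget after a delay.
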(event OnComponentBeginOverlap(Sphere)
  (params (OverlappedComponent :type Primitive%20Component%20Object%20Reference) (OtherActor :type Actor%20Object%20Reference) (OtherComp :type Primitive%20Component%20Object%20Reference) (OtherBodyIndex :type Integer) (bFromSweep :type Boolean) (SweepResult :type Hit%20Result%20Structure%20%28by%20ref%29))
  (bind _widget (Variables|Default|GetWidget))
  (Utilities|Casting|CastToBP_MCH OtherActor)
  (CallFunction|SetItemInfo (Variables|Default|GetName) (.quantity (Variables|Default|GetValues)))
  (Rendering|SetVisibility _widget true false)
  (bind _aswb_item_info (Utilities|Casting|CastToWB_ItemInfo (UserInterface|GetUserWidgetObject _widget)))
  (UserInterface|Animation|PlayAnimation _aswb_item_info (Variables|/Game/Equipment/UI_Blueprints/Components/WB_ItemInfo.WB_ItemInfo_C|GetUpAnimation _aswb_item_info) 0.0 1 "Forward" 1.0 false))

(event OnComponentEndOverlap(Sphere)
  (params (OverlappedComponent :type Primitive%20Component%20Object%20Reference) (OtherActor :type Actor%20Object%20Reference) (OtherComp :type Primitive%20Component%20Object%20Reference) (OtherBodyIndex :type Integer))
  (Utilities|Casting|CastToBP_MCH OtherActor)
  (UserInterface|Animation|PlayAnimation (stale OnComponentBeginOverlap(Sphere) _aswb_item_info) (Variables|/Game/Equipment/UI_Blueprints/Components/WB_ItemInfo.WB_ItemInfo_C|GetUpAnimation (stale OnComponentBeginOverlap(Sphere) _aswb_item_info)) 0.0 1 "Reverse" 1.0 false)
  (Utilities|FlowControl|Delay 1.0)
  (Rendering|SetVisibility (Variables|Default|GetWidget) false false))

(fn ConstructionScript
  (bind _values (Variables|Default|GetValues))
  (bind _itemdata (Variables|Default|GetitemData))
  (bind _item (Utilities|Struct|BreakS_Slot _itemdata))
  (bind (_datatable _rowname) (Utilities|Struct|BreakDataTableRowHandle _item))
  (Development|PrintString (Utilities|String|Append (Utilities|String|ToString(Integer) (.quality _values)) "     " (Utilities|String|ToString(Integer) (.quantity _values)) "     " (Utilities|String|ToString(Float) (.price _values))) true true "(R=1.000000,G=0.000000,B=0.090116,A=1.000000)" 5.0)
  (bind _returnvalue (Utilities|GetDataTableRow _datatable _rowname)
    (:then
      (Rendering|Components|Sprite|SetSprite (Variables|Default|GetPaperSprite) (.Sprite (Utilities|Struct|BreakS_MonsterItem _returnvalue)))
      (Variables|Default|SetName (.Name (Utilities|Struct|BreakS_MonsterItem _returnvalue)))
      (Transformation|SetRelativeScale3D (Variables|Default|GetSphere) "2.000000,2.000000,2.000000")
      (Transformation|SetRelativeScale3D (Variables|Default|GetPaperSprite) "1.500000,1.500000,1.500000"))))

(fn SetItemInfo
  (params (Name :type Text) (Quantity :type Integer))
  (bind _aswb_item_info (Utilities|Casting|CastToWB_ItemInfo (UserInterface|GetUserWidgetObject (Variables|Default|GetWidget))))
  (Variables|/Script/UMG.TextBlock|SetText (Variables|/Game/Equipment/UI_Blueprints/Components/WB_ItemInfo.WB_ItemInfo_C|GetName_Text _aswb_item_info) Name)
  (if (> Quantity 1)
    (Variables|/Script/UMG.TextBlock|SetText (Variables|/Game/Equipment/UI_Blueprints/Components/WB_ItemInfo.WB_ItemInfo_C|GetQuantity_Text _aswb_item_info) (Utilities|Text|ToText(String) (Utilities|String|Append (LocalVariables|Getthe%20X) (Utilities|String|ToString(Integer) Quantity))))))